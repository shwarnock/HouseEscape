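; An interactable key-locked door that swings open, then closes itself after a short delay.
; Its trigger box highlights the door through custom depth and shows a have-key or no-key widget based on the player's owned keys.
; Interacting inside the trigger with the required key drives timeline yaw rotation, with a Moving flag and DoOnce gating open and close.
; Dispatchers signal level loading during opening and unloading once closed.
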(event OnComponentEndOverlap(TriggerBox)
  (params (OverlappedComponent :type Primitive%20Component%20Object%20Reference) (OtherActor :type Actor%20Object%20Reference) (OtherComp :type Primitive%20Component%20Object%20Reference) (OtherBodyIndex :type Integer))
  ;[1 1 1] Remove UI when you leave the trigger
  (Utilities|Casting|CastToPlayerCharacter OtherActor)
  (Rendering|SetRenderCustomDepth (Variables|Default|GetDefaultMesh) false)
  (Rendering|SetRenderCustomDepth (Variables|Default|GetDoorFrame) false)
  (CallFunction|RemoveWidgets OtherActor))

(event OnComponentBeginOverlap(TriggerBox)
  (params (OverlappedComponent :type Primitive%20Component%20Object%20Reference) (OtherActor :type Actor%20Object%20Reference) (OtherComp :type Primitive%20Component%20Object%20Reference) (OtherBodyIndex :type Integer) (bFromSweep :type Boolean) (SweepResult :type Hit%20Result%20Structure%20%28by%20ref%29))
  ;[1 1 1] Displays UI telling the player to find a key or open the door when entering the trigger volume
  (Utilities|Casting|CastToPlayerCharacter OtherActor)
  (CallFunction|DisplayUI)
  (Rendering|SetRenderCustomDepth (Variables|Default|GetDefaultMesh) true)
  (Rendering|SetRenderCustomDepth (Variables|Default|GetDoorFrame) true))

(event Custom|CloseDoor
  ;[1 1 1] Close Door
  (Utilities|FlowControl|Delay (Math|Random|RandomFloatinRange 2.0 2.0))
  (if (not (Variables|Default|GetMoving?))
    (Utilities|FlowControl|DoOnce false
      (:Completed
        (Variables|Default|SetMoving? true)
        (bind _newtrack_0 (Timeline|Timeline_1 ReverseFromEnd)
          (:Update
            (Transformation|SetRelativeRotation (Variables|Default|GetDefaultMesh) (Math|Rotator|MakeRotator 0.0 0.0 (* _newtrack_0 (Variables|Default|GetZ))) false false))
          (:Finished
            (Variables|Default|SetClosed? true)
            (Variables|Default|SetMoving? false)
            (Default|CallUnloadLevelDispatcher self)))))))

(event EventOnInteract
  (params (Instigator :type Player%20Character%20Object%20Reference))
  ;[1 1 1] Check Overlap
  (if (not (Variables|Default|GetMoving?))
    (bind _newparam (CallFunction|CheckPlayerOverlap))
    (if _newparam
      ;[1 1 1] Check to see if the player has the required keys
      (bind _asplayer_character (Utilities|Casting|CastToPlayerCharacter (Game|GetPlayerCharacter 0)))
      (for _array_element (Variables|/Game/Blueprints/Characters/PlayerCharacter.PlayerCharacter_C|GetOwnedKeys _asplayer_character)
        (if (Utilities|Enum|Equal(Enum) _array_element (Variables|Default|GetRequiredKeys))
          (if (Variables|Default|GetClosed?)
            (Utilities|FlowControl|Sequence
              (:then_0
                (Variables|Default|SetMoving? true)
                ;[1 1 1] Open Door
                (bind _newtrack_0 (Timeline|Timeline_0 PlayFromStart)
                  (:Update
                    (Transformation|SetRelativeRotation (Variables|Default|GetDefaultMesh) (Math|Rotator|MakeRotator 0.0 0.0 (* _newtrack_0 (Variables|Default|GetZ))) false false)
                    (bind _foundwidgets (Widget|GetAllWidgetsOfClass "/Game/UI/DoorWidgetHaveKey.DoorWidgetHaveKey_C" true))
                    (Widget|RemovefromParent _foundwidgets)
                    (Default|CallLoadLevelDispatcher self))
                  (:Finished
                    (Variables|Default|SetClosed? false)
                    (Variables|Default|SetMoving? false)
                    (CallFunction|CloseDoor))))
              (:then_1
                (goto _label Reset)))
            (else
              ;[1 1 1] Close Door
              (Utilities|FlowControl|DoOnce false :!label _label
                (:Completed
                  (Variables|Default|SetMoving? true)
                  (bind _newtrack_0_2 (Timeline|Timeline_1 ReverseFromEnd)
                    (:Update
                      (Transformation|SetRelativeRotation (Variables|Default|GetDefaultMesh) (Math|Rotator|MakeRotator 0.0 0.0 (* _newtrack_0_2 (Variables|Default|GetZ))) false false))
                    (:Finished
                      (Variables|Default|SetClosed? true)
                      (Variables|Default|SetMoving? false)
                      (Default|CallUnloadLevelDispatcher self))))))))))))

(fn ConstructionScript)

(fn RemoveWidgets
  (params (OverlappingActor :type Actor%20Object%20Reference))
  (if (== OverlappingActor (Game|GetPlayerCharacter 0))
    (Viewport|RemoveAllWidgets)))

(fn DisplayUI
  (bind _asplayer_character (Utilities|Casting|CastToPlayerCharacter (Game|GetPlayerCharacter 0)))
  (bind _array_element (Utilities|Array|ForEachLoopwithBreak (Variables|/Game/Blueprints/Characters/PlayerCharacter.PlayerCharacter_C|GetOwnedKeys _asplayer_character) :!label _label)
    (:LoopBody
      (if (Utilities|Enum|Equal(Enum) _array_element (Variables|Default|GetRequiredKeys))
        (Variables|Default|SetHaveKey? true)
        (goto _label Break)))
    (:Completed
      (if (Variables|Default|GetHaveKey?)
        (if (Variables|Default|GetClosed?)
          (bind _foundwidgets (Widget|GetAllWidgetsOfClass "/Game/UI/DoorWidgetNoKey.DoorWidgetNoKey_C" true))
          (Widget|RemovefromParent _foundwidgets)
          (bind _returnvalue (UserInterface|CreateWidget "/Game/UI/DoorWidgetHaveKey.DoorWidgetHaveKey_C"))
          (UserInterface|Viewport|AddtoViewport _returnvalue 0))
        (else
          (bind _returnvalue_2 (UserInterface|CreateWidget "/Game/UI/DoorWidgetNoKey.DoorWidgetNoKey_C"))
          (UserInterface|Viewport|AddtoViewport _returnvalue_2 0))))))

(fn CheckPlayerOverlap
  (return (Class|PrimitiveComponent|IsOverlappingComponent (Variables|/Script/Engine.Character|GetCapsuleComponent (Game|GetPlayerCharacter 0)) (Variables|Default|GetTriggerBox))))

(fn LoadNextLevel)