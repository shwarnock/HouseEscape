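; Light actor that flickers a point light on and off at random intervals during play.
; BeginPlay starts an endless loop that waits a random delay of up to one second, then toggles PointLight visibility and the LightOn flag.
; The construction script applies the actor's Intensity, AttenuationRadius and SourceRadius variables to the point light.
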(event EventBeginPlay
  (Utilities|FlowControl|RetriggerableDelay (Math|Random|RandomFloatinRange 0.0 1.0) :!label _label)
  (if (Variables|Default|GetLightOn?)
    (Rendering|SetVisibility (Variables|Default|GetPointLight) false false)
    (Variables|Default|SetLightOn? false)
    (goto _label)
    (else
      (Rendering|SetVisibility (Variables|Default|GetPointLight) true false)
      (Variables|Default|SetLightOn? true)
      (goto _label))))

(fn ConstructionScript
  (Rendering|Components|Light|SetIntensity (Variables|Default|GetPointLight) (Variables|Default|GetIntensity))
  (Rendering|Lighting|SetAttenuationRadius (Variables|Default|GetPointLight) (Variables|Default|GetAttenuationRadius))
  (Class|PointLightComponent|SetSourceRadius (Variables|Default|GetPointLight) (Variables|Default|GetSourceRadius)))