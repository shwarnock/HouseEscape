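; BaseItem is a pickup item Actor that hands its ItemInfo to the interacting instigator's Pickup function, then destroys itself.
; A sphere overlap with PlayerCharacter enables custom depth on the mesh and adds an interact widget to the viewport.
; Leaving the sphere disables custom depth and removes all widgets, not just its own prompt.
; The construction script writes the actor's own class into ItemInfo, preserving the other fields.
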(event OnComponentBeginOverlap(Sphere)
  (params (OverlappedComponent :type Primitive%20Component%20Object%20Reference) (OtherActor :type Actor%20Object%20Reference) (OtherComp :type Primitive%20Component%20Object%20Reference) (OtherBodyIndex :type Integer) (bFromSweep :type Boolean) (SweepResult :type Hit%20Result%20Structure%20%28by%20ref%29))
  (Utilities|Casting|CastToPlayerCharacter OtherActor)
  (Rendering|SetRenderCustomDepth (Variables|Default|GetStaticMesh) true)
  (bind _returnvalue (UserInterface|CreateWidget "/Game/UI/InteractWidget.InteractWidget_C"))
  (UserInterface|Viewport|AddtoViewport _returnvalue 0))

(event OnComponentEndOverlap(Sphere)
  (params (OverlappedComponent :type Primitive%20Component%20Object%20Reference) (OtherActor :type Actor%20Object%20Reference) (OtherComp :type Primitive%20Component%20Object%20Reference) (OtherBodyIndex :type Integer))
  (Utilities|Casting|CastToPlayerCharacter OtherActor)
  (Rendering|SetRenderCustomDepth (Variables|Default|GetStaticMesh) false)
  (Viewport|RemoveAllWidgets))

(event EventOnInteract
  (params (Instigator :type Player%20Character%20Object%20Reference))
  (Default|Pickup Instigator (Variables|Default|GetItemInfo))
  (Actor|DestroyActor))

(fn ConstructionScript
  (Variables|Default|SetItemInfo (Utilities|Struct|MakeItemInfo (.itemtype (Variables|Default|GetItemInfo)) (.itemname (Variables|Default|GetItemInfo)) (.itemimage (Variables|Default|GetItemInfo)) (.itemindex (Variables|Default|GetItemInfo)) (Utilities|GetClass self))))