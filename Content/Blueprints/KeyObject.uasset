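; A key pickup actor that, on interact, adds its key type to the player character's owned keys and destroys itself.
; The interaction only succeeds while the actor overlaps the player character.
; Trigger box overlap events are empty; the logic for toggling a custom-depth highlight and UI widget on the player's approach is disconnected and never runs.
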(event OnComponentBeginOverlap(TriggerBox)
  (params (OverlappedComponent :type Primitive%20Component%20Object%20Reference) (OtherActor :type Actor%20Object%20Reference) (OtherComp :type Primitive%20Component%20Object%20Reference) (OtherBodyIndex :type Integer) (bFromSweep :type Boolean) (SweepResult :type Hit%20Result%20Structure%20%28by%20ref%29))
  ;[1 1 1] Add and remove UI from Viewport
)

(event OnComponentEndOverlap(TriggerBox)
  (params (OverlappedComponent :type Primitive%20Component%20Object%20Reference) (OtherActor :type Actor%20Object%20Reference) (OtherComp :type Primitive%20Component%20Object%20Reference) (OtherBodyIndex :type Integer))
  ;[1 1 1] Add and remove UI from Viewport
)

(event EventOnInteract
  (params (Instigator :type Player%20Character%20Object%20Reference))
  ;[1 1 1] Add Key to Owned Keys
  (if (Collision|IsOverlappingActor (Game|GetPlayerCharacter 0) :!class /Script/Engine.Actor)
    (bind _asplayer_character (Utilities|Casting|CastToPlayerCharacter (Game|GetPlayerCharacter 0)))
    (Utilities|Array|Add (Variables|/Game/Blueprints/Characters/PlayerCharacter.PlayerCharacter_C|GetOwnedKeys _asplayer_character) (Variables|Default|GetKeyType))
    (Actor|DestroyActor)))

(fn ConstructionScript)