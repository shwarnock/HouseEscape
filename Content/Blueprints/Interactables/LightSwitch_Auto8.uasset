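; Interactable light switch for a light puzzle that can award a key.
; Interacting toggles one or two linked lights and records the primary light's name in the Game Instance's LightsOn list.
; If the player lacks the puzzle's key, it spawns one at a fixed location when Light1, Light3 and Light5 are absent from that list.
; Box overlap shows or removes the interact widget and custom-depth highlight.
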(event OnComponentBeginOverlap(Box)
  (params (OverlappedComponent :type Primitive%20Component%20Object%20Reference) (OtherActor :type Actor%20Object%20Reference) (OtherComp :type Primitive%20Component%20Object%20Reference) (OtherBodyIndex :type Integer) (bFromSweep :type Boolean) (SweepResult :type Hit%20Result%20Structure%20%28by%20ref%29))
  (CallFunction|CreateUI OtherActor))

(event OnComponentEndOverlap(Box)
  (params (OverlappedComponent :type Primitive%20Component%20Object%20Reference) (OtherActor :type Actor%20Object%20Reference) (OtherComp :type Primitive%20Component%20Object%20Reference) (OtherBodyIndex :type Integer))
  (CallFunction|RemoveUI OtherActor))

(event EventOnInteract
  (CallFunction|ToggleLight)
  (bind _ownkey_ (CallFunction|DoesPlayerOwnKey?))
  (if (not _ownkey_)
    (CallFunction|CheckSolution)))

(fn ConstructionScript)

(fn ToggleLight
  (bind _light2 (Variables|Default|GetLight2))
  (bind _light2_2 (Variables|Default|GetLight2))
  (if (Variables|Default|GetLightOn?)
    (Rendering|ToggleVisibility (Variables|/Script/Engine.PointLight|GetPointLightComponent (Variables|Default|GetLight)) false)
    (bind _asmy_game_instance (Utilities|Casting|CastTo (Game|GetGameInstance)))
    (Utilities|Array|RemoveItem (Variables|Default|GetLightsOn _asmy_game_instance) (Utilities|GetDisplayName (Variables|Default|GetLight)))
    (Variables|Default|SetLightOn? false)
    (Utilities|IsValid _light2_2
      (:Is%20Valid
        (Rendering|ToggleVisibility (Variables|/Script/Engine.PointLight|GetPointLightComponent _light2_2) false)))
    (else
      (Rendering|ToggleVisibility (Variables|/Script/Engine.Light|GetLightComponent (Variables|Default|GetLight)) false)
      (bind _asmy_game_instance_2 (Utilities|Casting|CastTo (Game|GetGameInstance)))
      (Utilities|Array|Add (Variables|Default|GetLightsOn _asmy_game_instance_2) (Utilities|GetDisplayName (Variables|Default|GetLight)))
      (Variables|Default|SetLightOn? true)
      (Utilities|IsValid _light2
        (:Is%20Valid
          (Rendering|ToggleVisibility (Variables|/Script/Engine.Light|GetLightComponent _light2) false))))))

(fn DoesPlayerOwnKey?
  (bind _asplayer_character (Utilities|Casting|CastToPlayerCharacter (Game|GetPlayerCharacter 0)))
  (bind _array_element (Utilities|Array|ForEachLoopwithBreak (Variables|/Game/Blueprints/Characters/PlayerCharacter.PlayerCharacter_C|GetOwnedKeys _asplayer_character) :!label _label)
    (:LoopBody
      (if (Utilities|Enum|Equal(Enum) _array_element "NewEnumerator14")
        (LocalVariables|SetLocalOwnKey? true)
        (goto _label Break)))
    (:Completed
      (return (LocalVariables|GetLocalOwnKey?)))))

(fn CheckSolution
  (bind _asmy_game_instance (Utilities|Casting|CastTo (Game|GetGameInstance)))
  (bind _array_element (Utilities|Array|ForEachLoopwithBreak (Variables|Default|GetLightsOn _asmy_game_instance) :!label _label)
    (:LoopBody
      (if (Math|Boolean|ORBoolean (Utilities|Enum|Equal(Enum) _array_element "Light3") (Utilities|Enum|Equal(Enum) _array_element "Light1") (Utilities|Enum|Equal(Enum) _array_element "Light5"))
        (LocalVariables|SetWrong? true)
        (goto _label Break)))
    (:Completed
      (if (not (LocalVariables|GetWrong?))
        (bind _returnvalue (Game|SpawnActorfromClass "/Game/Blueprints/KeyObject.KeyObject_C" (Math|Transform|MakeTransform "2720.000000,-2775.000000,-285.000000" "0, 0, 0" "1,1,1") "Undefined" 0 0))
        (Variables|/Game/Blueprints/KeyObject.KeyObject_C|SetKeyType _returnvalue "NewEnumerator14")))))

(fn RemoveUI
  (params (Object :type Object%20Object%20Reference))
  (Utilities|Casting|CastToPlayerCharacter Object)
  (Viewport|RemoveAllWidgets)
  (Rendering|SetRenderCustomDepth (Variables|Default|GetStaticMesh) false))

(fn CreateUI
  (params (Object :type Object%20Object%20Reference))
  (Utilities|Casting|CastToPlayerCharacter Object)
  (bind _returnvalue (UserInterface|CreateWidget "/Game/UI/InteractWidget.InteractWidget_C"))
  (UserInterface|Viewport|AddtoViewport _returnvalue 0)
  (Rendering|SetRenderCustomDepth (Variables|Default|GetStaticMesh) true))