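; AI controller that runs a behavior tree to hunt the player, feeding it sight state through blackboard keys from AI Perception.
; A 0.2-second loop samples random floor-tagged TargetPoints to update PathingNode, aiming for points near the player.
; MoveAI teleports an unaware, distant or other-floor pawn to a random point near the player, filtered by screen-projection and line-trace visibility checks, then toggles ActorMoved.
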(event OnTargetPerceptionUpdated(AIPerception)
  (params (Actor :type Actor%20Object%20Reference) (Stimulus :type AI%20Stimulus%20Structure))
  (bind (_age _expirationage _strength _stimuluslocation _receiverlocation _tag _bsuccessfullysensed) (Utilities|Struct|BreakAIStimulus Stimulus))
  (bind _returnvalue (Game|GetPlayerCharacter 0))
  (bind _self self)
  (bind _returnvalue_2 (AI|GetBlackboard _self))
  ;[1 1 1] Move AI to Player (Working)
  (if (== Actor _returnvalue)
    (if _bsuccessfullysensed
      (Variables|Default|SetDoesAISeeEnemy true)
      (AI|Components|Blackboard|SetValueasObject _returnvalue_2 (Variables|Default|GetEnemyActorKeyName) _returnvalue)
      (else
        (Variables|Default|SetDoesAISeeEnemy false)
        (AI|Components|Blackboard|SetValueasVector _returnvalue_2 (Utilities|Name|MakeLiteralName "LastKnownPosition") _stimuluslocation)))))

(event Custom|MoveAI
  (bind _returnvalue (Game|GetPlayerController 0))
  (bind _returnvalue_2 (Game|Player|GetPlayerPawn 0))
  (bind _goodnodes (Variables|Default|GetGoodNodes))
  (bind _returnvalue_3 (Utilities|Array|Length _goodnodes))
  (bind _returnvalue_4 (Viewport|GetViewportSize _returnvalue))
  (if (not (Variables|Default|GetDoesAISeeEnemy))
    ;[1 1 1] Line trace between player and target point
    (if (or (> (Math|Float|Absolute(Float) (- (.z (Transformation|GetActorLocation (Pawn|GetControlledPawn))) (.z (Transformation|GetActorLocation (Game|Player|GetPlayerPawn 0))))) 2e+02) (> (Transformation|GetDistanceTo (Game|Player|GetPlayerPawn 0)) 3e+03))
      (bind _array_element (Utilities|Array|ForEachLoopwithBreak (Variables|Default|GetPathingNodeArray))
        (:LoopBody
          (bind _output_get (Variables|Default|SetCurrentNode _array_element))
          (bind _outhit (Collision|LineTraceByChannel (Transformation|GetActorLocation (Game|Player|GetPlayerPawn 0)) (Transformation|GetActorLocation _output_get) "TraceTypeQuery1" false 0 "ForOneFrame"))
          (if (or (Math|Boolean|NANDBoolean (> (.x (.ScreenLocation (Class|PlayerController|ProjectWorldLocationtoScreen _returnvalue (Transformation|GetActorLocation (Variables|Default|GetCurrentNode)) false))) 0.0) (> (.y (.ScreenLocation (Class|PlayerController|ProjectWorldLocationtoScreen _returnvalue (Transformation|GetActorLocation (Variables|Default|GetCurrentNode)) false))) 0.0) (< (.x (.ScreenLocation (Class|PlayerController|ProjectWorldLocationtoScreen _returnvalue (Transformation|GetActorLocation (Variables|Default|GetCurrentNode)) false))) (.x _returnvalue_4)) (< (.x (.ScreenLocation (Class|PlayerController|ProjectWorldLocationtoScreen _returnvalue (Transformation|GetActorLocation (Variables|Default|GetCurrentNode)) false))) (.y _returnvalue_4))) (!= (.HitActor (Collision|BreakHitResult _outhit)) (Variables|Default|GetCurrentNode)))
            (if (Math|Boolean|ANDBoolean (< (Math|Float|Absolute(Float) (- (.z (Transformation|GetActorLocation (Variables|Default|GetCurrentNode))) (.z (Transformation|GetActorLocation _returnvalue_2)))) 1e+02) (> (Transformation|GetDistanceTo (Variables|Default|GetCurrentNode) _returnvalue_2) 5e+02) (< (Transformation|GetDistanceTo (Variables|Default|GetCurrentNode) _returnvalue_2) 2e+03))
              (Utilities|Array|Add (Variables|Default|GetGoodNodes) (Variables|Default|GetCurrentNode)))))
        (:Completed
          (if (> _returnvalue_3 0)
            (Transformation|SetActorLocation (Pawn|GetControlledPawn) (Transformation|GetActorLocation (Utilities|Array|Get(acopy) _goodnodes (Math|Random|RandomInteger _returnvalue_3))) false false)
            (Utilities|Array|Clear (Variables|Default|GetGoodNodes))
            (Development|PrintString "Move Occurred")
            (Utilities|FlowControl|FlipFlop
              (:A
                (Variables|Default|SetActorMoved? true))
              (:B
                (bind _output_get_2 (Variables|Default|SetActorMoved? false))))
            (AI|Components|Blackboard|SetValueasBool (AI|GetBlackboard self) (Utilities|Name|MakeLiteralName "ActorMoved") _output_get_2)))))))

(event EventBeginPlay
  (bind _pathingnodearray (Variables|Default|GetPathingNodeArray))
  ;[1 1 1] Start Behavior Tree
  (AI|RunBehaviorTree "/Game/Blueprints/Characters/AIBehaviorTree.AIBehaviorTree")
  ;[1 1 1] Initialize Pathing Node Array
  (bind _outactors (Actor|GetAllActorsOfClass "/Script/Engine.TargetPoint"))
  (for _array_element _outactors
    (if (or (Actor|ActorHasTag _array_element "SecondFloor") (Actor|ActorHasTag _array_element "FirstFloor"))
      (Utilities|Array|Add (Variables|Default|GetPathingNodeArray) _array_element)))
  (Utilities|FlowControl|Sequence :!label _label
    (:then_0
      ;[1 1 1] Check for valid target point
      (bind _output_get (Variables|Default|SetCurrentNodeBlackBoard (Utilities|Array|Get(acopy) _pathingnodearray (Math|Random|RandomInteger (Utilities|Array|Length _pathingnodearray)))))
      (if (not (or (> (Transformation|GetDistanceTo (Game|Player|GetPlayerPawn 0) _output_get) 2e+03) (> (Math|Float|Absolute(Float) (- (.z (Transformation|GetActorLocation _output_get)) (.z (Transformation|GetActorLocation (Game|Player|GetPlayerPawn 0))))) 5e+01)))
        (Variables|Default|SetHaveGoodNode? true)))
    (:then_1
      ;[1 1 1] Set current node as blackboard value
      (if (Variables|Default|GetHaveGoodNode?)
        (AI|Components|Blackboard|SetValueasObject (AI|GetBlackboard self) (Utilities|Name|MakeLiteralName "PathingNode") (Variables|Default|GetCurrentNodeBlackBoard))))
    (:then_2
      (Utilities|FlowControl|RetriggerableDelay 0.2)
      (goto _label))))

(fn ConstructionScript)