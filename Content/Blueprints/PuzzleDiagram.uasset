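; PuzzleDiagram is an interactable actor in a house escape game that the player can switch the camera to.
; Its box overlap adds and removes an interact target through the HouseEscapeGameInstance's messenger as the HouseEscapeCharacter enters and leaves.
; OnInteract toggles the player controller's view target between this actor and the player character with a short blend.
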(event OnComponentBeginOverlap(BoxComponent)
  (params (OverlappedComponent :type Primitive%20Component%20Object%20Reference) (OtherActor :type Actor%20Object%20Reference) (OtherComp :type Primitive%20Component%20Object%20Reference) (OtherBodyIndex :type Integer) (bFromSweep :type Boolean) (SweepResult :type Hit%20Result%20Structure%20%28by%20ref%29))
  (Utilities|Casting|CastToHouseEscapeCharacter OtherActor)
  (bind _ashouse_escape_game_instance (Utilities|Casting|CastToHouseEscapeGameInstance (Game|GetGameInstance)))
  (bind _returnvalue (Class|HouseEscapeGameInstance|GetMessenger _ashouse_escape_game_instance))
  (Class|Messenger|AddInteractTarget _returnvalue (Utilities|Struct|MakeMessage "(itemType=Screwdriver,texture=None,name=\"\",itemIndex=0,baseClass=None)" (Utilities|Array|MakeArray ""))))

(event OnComponentEndOverlap(BoxComponent)
  (params (OverlappedComponent :type Primitive%20Component%20Object%20Reference) (OtherActor :type Actor%20Object%20Reference) (OtherComp :type Primitive%20Component%20Object%20Reference) (OtherBodyIndex :type Integer))
  (Utilities|Casting|CastToHouseEscapeCharacter OtherActor)
  (bind _ashouse_escape_game_instance (Utilities|Casting|CastToHouseEscapeGameInstance (Game|GetGameInstance)))
  (bind _returnvalue (Class|HouseEscapeGameInstance|GetMessenger _ashouse_escape_game_instance))
  (Class|Messenger|RemoveInteractTarget _returnvalue (Utilities|Struct|MakeMessage "(itemType=Screwdriver,texture=None,name=\"\",itemIndex=0,baseClass=None)" (Utilities|Array|MakeArray ""))))

(event EventOnInteract
  (bind _returnvalue (Game|GetPlayerController 0))
  (bind _self self)
  (if (== (Pawn|GetViewTarget _returnvalue) _self)
    (Game|Player|SetViewTargetwithBlend _returnvalue (Game|GetPlayerCharacter 0) 0.5 "VTBlend_Linear" 0.0 false)
    (else
      (Game|Player|SetViewTargetwithBlend _returnvalue _self 0.5 "VTBlend_Linear" 0.0 false))))

(fn ConstructionScript)