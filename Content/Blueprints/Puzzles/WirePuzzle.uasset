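; Wire puzzle actor where the player clicks eight nodes to cycle their colors until each lettered pair shows its named color.
; Interacting inside the trigger toggles a camera change and mouse click input through a FlipFlop.
; Each click runs SetColor, storing the node's color index, then CheckSolution, which spawns a key and marks the puzzle solved.
; On BeginPlay, an already-owned key displays the solved colors and disables interaction.
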(event OnClicked(RedB)
  (params (TouchedComponent :type Primitive%20Component%20Object%20Reference) (ButtonPressed :type Key%20Structure :default "AnyKey"))
  ;[1 1 1] Change Node colors on mouse click
  (bind _outputint (CallFunction|SetColor TouchedComponent (Variables|Default|GetRedB_Int)))
  (Variables|Default|SetRedB_Int _outputint)
  (CallFunction|CheckSolution))

(event OnComponentBeginOverlap(Trigger)
  (params (OverlappedComponent :type Primitive%20Component%20Object%20Reference) (OtherActor :type Actor%20Object%20Reference) (OtherComp :type Primitive%20Component%20Object%20Reference) (OtherBodyIndex :type Integer) (bFromSweep :type Boolean) (SweepResult :type Hit%20Result%20Structure%20%28by%20ref%29))
  ;[1 1 1] Add and Remove UI
  (if (not (Variables|Default|GetHaveKey?))
    (Rendering|SetRenderCustomDepth (Variables|Default|GetStaticMesh) true)
    (bind _returnvalue (UserInterface|CreateWidget "/Game/UI/InteractWidget.InteractWidget_C"))
    (UserInterface|Viewport|AddtoViewport _returnvalue 0)))

(event OnComponentEndOverlap(Trigger)
  (params (OverlappedComponent :type Primitive%20Component%20Object%20Reference) (OtherActor :type Actor%20Object%20Reference) (OtherComp :type Primitive%20Component%20Object%20Reference) (OtherBodyIndex :type Integer))
  ;[1 1 1] Add and Remove UI
  (Viewport|RemoveAllWidgets)
  (Rendering|SetRenderCustomDepth (Variables|Default|GetStaticMesh) false))

(event OnClicked(RedA)
  (params (TouchedComponent :type Primitive%20Component%20Object%20Reference) (ButtonPressed :type Key%20Structure :default "AnyKey"))
  ;[1 1 1] Change Node colors on mouse click
  (bind _outputint (CallFunction|SetColor TouchedComponent (Variables|Default|GetRedA_Int)))
  (Variables|Default|SetRedA_Int _outputint)
  (CallFunction|CheckSolution))

(event OnClicked(GreenA)
  (params (TouchedComponent :type Primitive%20Component%20Object%20Reference) (ButtonPressed :type Key%20Structure :default "AnyKey"))
  ;[1 1 1] Change Node colors on mouse click
  (bind _outputint (CallFunction|SetColor TouchedComponent (Variables|Default|GetGreenA_Int)))
  (Variables|Default|SetGreenA_Int _outputint)
  (CallFunction|CheckSolution))

(event OnClicked(YellowA)
  (params (TouchedComponent :type Primitive%20Component%20Object%20Reference) (ButtonPressed :type Key%20Structure :default "AnyKey"))
  ;[1 1 1] Change Node colors on mouse click
  (bind _outputint (CallFunction|SetColor TouchedComponent (Variables|Default|GetYellowA_Int)))
  (Variables|Default|SetYellowA_Int _outputint)
  (CallFunction|CheckSolution))

(event OnClicked(YellowB)
  (params (TouchedComponent :type Primitive%20Component%20Object%20Reference) (ButtonPressed :type Key%20Structure :default "AnyKey"))
  ;[1 1 1] Change Node colors on mouse click
  (bind _outputint (CallFunction|SetColor TouchedComponent (Variables|Default|GetYellowB_Int)))
  (Variables|Default|SetYellowB_Int _outputint)
  (CallFunction|CheckSolution))

(event OnClicked(GreenB)
  (params (TouchedComponent :type Primitive%20Component%20Object%20Reference) (ButtonPressed :type Key%20Structure :default "AnyKey"))
  ;[1 1 1] Change Node colors on mouse click
  (bind _outputint (CallFunction|SetColor TouchedComponent (Variables|Default|GetGreenB_Int)))
  (Variables|Default|SetGreenB_Int _outputint)
  (CallFunction|CheckSolution))

(event OnClicked(BlueA)
  (params (TouchedComponent :type Primitive%20Component%20Object%20Reference) (ButtonPressed :type Key%20Structure :default "AnyKey"))
  ;[1 1 1] Change Node colors on mouse click
  (bind _outputint (CallFunction|SetColor TouchedComponent (Variables|Default|GetBlueA_Int)))
  (Variables|Default|SetBlueA_Int _outputint)
  (CallFunction|CheckSolution))

(event OnClicked(BlueB)
  (params (TouchedComponent :type Primitive%20Component%20Object%20Reference) (ButtonPressed :type Key%20Structure :default "AnyKey"))
  ;[1 1 1] Change Node colors on mouse click
  (bind _outputint (CallFunction|SetColor TouchedComponent (Variables|Default|GetBlueB_Int)))
  (Variables|Default|SetBlueB_Int _outputint)
  (CallFunction|CheckSolution))

(event EventBeginPlay
  ;[1 1 1] Check to See if puzzle was solved
  (bind _asplayer_character (Utilities|Casting|CastToPlayerCharacter (Game|GetPlayerCharacter 0)))
  (bind _array_element (Utilities|Array|ForEachLoopwithBreak (Variables|/Game/Blueprints/Characters/PlayerCharacter.PlayerCharacter_C|GetOwnedKeys _asplayer_character) :!label _label)
    (:LoopBody
      (if (Utilities|Enum|Equal(Enum) _array_element "NewEnumerator9")
        (Variables|Default|SetHaveKey? true)
        (goto _label Break)))
    (:Completed
      (if (Variables|Default|GetHaveKey?)
        (Utilities|FlowControl|Sequence
          (:then_0
            (Rendering|Material|SetMaterial (Variables|Default|GetGreenB) 0 "/Game/Materials/WirePuzzke/Green.Green")
            (Rendering|Material|SetMaterial (Variables|Default|GetYellowB) 0 "/Game/Materials/WirePuzzke/Yellow.Yellow")
            (Rendering|Material|SetMaterial (Variables|Default|GetBlueB) 0 "/Game/Materials/WirePuzzke/Blue.Blue")
            (Rendering|Material|SetMaterial (Variables|Default|GetYellowA) 0 "/Game/Materials/WirePuzzke/Yellow.Yellow"))
          (:then_1
            (Rendering|Material|SetMaterial (Variables|Default|GetGreenA) 0 "/Game/Materials/WirePuzzke/Green.Green")
            (Rendering|Material|SetMaterial (Variables|Default|GetRedA) 0 "/Game/Materials/WirePuzzke/Red.Red")
            (Rendering|Material|SetMaterial (Variables|Default|GetRedB) 0 "/Game/Materials/WirePuzzke/Red.Red")
            (Rendering|Material|SetMaterial (Variables|Default|GetBlueA) 0 "/Game/Materials/WirePuzzke/Blue.Blue")))))))

(event EventOnInteract
  (params (Instigator :type Player%20Character%20Object%20Reference))
  (bind _returnvalue (Game|GetPlayerController 0))
  (bind _returnvalue_2 (Game|GetPlayerController 0))
  ;[1 1 1] Set Camera and Enable Mouse Click Inputs
  (if (not (Variables|Default|GetHaveKey?))
    (if (Class|PrimitiveComponent|IsOverlappingComponent (Variables|/Script/Engine.Character|GetCapsuleComponent (Game|GetPlayerCharacter 0)) (Variables|Default|GetTrigger))
      (Viewport|RemoveAllWidgets)
      (Utilities|FlowControl|FlipFlop
        (:A
          (Rendering|SetRenderCustomDepth (Variables|Default|GetStaticMesh) false)
          (Default|CallSetCamera)
          (Variables|/Script/Engine.PlayerController|SetbShowMouseCursor _returnvalue_2 true)
          (Variables|/Script/Engine.PlayerController|SetbEnableMouseOverEvents _returnvalue_2 true)
          (Variables|/Script/Engine.PlayerController|SetbEnableClickEvents _returnvalue_2 true)
          (Input|SetInputModeGameandUI _returnvalue_2 0 "DoNotLock" true))
        (:B
          (Default|CallSetCamera)
          (Utilities|FlowControl|Delay 0.5)
          (if (Variables|Default|GetSolved?)
            _
            (else
              (Rendering|SetRenderCustomDepth (Variables|Default|GetStaticMesh) true)))
          (Variables|/Script/Engine.PlayerController|SetbShowMouseCursor _returnvalue false)
          (Variables|/Script/Engine.PlayerController|SetbEnableMouseOverEvents _returnvalue false)
          (Variables|/Script/Engine.PlayerController|SetbEnableClickEvents _returnvalue false)
          (Input|SetInputModeGameOnly _returnvalue))))))

(fn ConstructionScript)

(fn SetColor
  (params (StaticMeshComponent :type Primitive%20Component%20Object%20Reference) (IntValue :type Integer))
  (LocalVariables|SetLocalMeshComponent StaticMeshComponent)
  (bind _output_get (LocalVariables|SetLocalInt IntValue))
  (if (== _output_get 3)
    (LocalVariables|SetLocalInt 0)
    (else
      (LocalVariables|SetLocalInt (+ (LocalVariables|GetLocalInt) 1))))
  (Utilities|FlowControl|MultiGate false false (LocalVariables|GetLocalInt)
    (:Out%200
      (Rendering|Material|SetMaterial (LocalVariables|GetLocalMeshComponent) 0 "/Game/Materials/WirePuzzke/Blue.Blue")
      (LocalVariables|SetLocalInt 0))
    (:Out%201
      (Rendering|Material|SetMaterial (LocalVariables|GetLocalMeshComponent) 0 "/Game/Materials/WirePuzzke/Red.Red")
      (LocalVariables|SetLocalInt 1))
    (:Out%202
      (Rendering|Material|SetMaterial (LocalVariables|GetLocalMeshComponent) 0 "/Game/Materials/WirePuzzke/Green.Green")
      (LocalVariables|SetLocalInt 2))
    (:Out%203
      (Rendering|Material|SetMaterial (LocalVariables|GetLocalMeshComponent) 0 "/Game/Materials/WirePuzzke/Yellow.Yellow")
      (LocalVariables|SetLocalInt 3)))
  (return (LocalVariables|GetLocalInt)))

(fn CheckSolution
  (if (and (== (Variables|Default|GetBlueA_Int) 0) (== (Variables|Default|GetBlueB_Int) 0))
    (if (and (== 1 (Variables|Default|GetRedA_Int)) (== 1 (Variables|Default|GetRedB_Int)))
      (if (and (== (Variables|Default|GetGreenA_Int) 2) (== (Variables|Default|GetGreenB_Int) 2))
        (if (and (== (Variables|Default|GetYellowA_Int) 3) (== (Variables|Default|GetYellowB_Int) 3))
          (bind _returnvalue (Game|SpawnActorfromClass "/Game/Blueprints/KeyObject.KeyObject_C" (Math|Transform|MakeTransform "1330.000000,-2075.000000,-290.000000" "0, 0,0.000000" "0.300000,0.300000,0.300000") "Undefined" 0 0))
          (Variables|/Game/Blueprints/KeyObject.KeyObject_C|SetKeyType _returnvalue "NewEnumerator9")
          (Variables|Default|SetSolved? true))))))