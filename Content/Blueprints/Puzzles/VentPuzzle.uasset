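; Vent puzzle actor where the player unscrews four screws with the screwdriver to open a vent and spawn a key.
; Interacting inside the trigger toggles the puzzle camera and mouse click input, and hovered screws highlight through custom depth.
; A clicked screw is destroyed only if the game instance's last clicked item is the screwdriver; removing all four destroys the cube cover.
; On BeginPlay, an already-owned key removes the cover and screws.
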(event OnClicked(Screw)
  (params (TouchedComponent :type Primitive%20Component%20Object%20Reference) (ButtonPressed :type Key%20Structure :default "AnyKey"))
  ;[1 1 1] Check to see if player has screwdriver equipped. If so delete screw.
  (CallFunction|DestroyScrew (Variables|Default|GetScrew))
  (CallFunction|CheckAllScrewsDestroyed))

(event OnClicked(Screw3)
  (params (TouchedComponent :type Primitive%20Component%20Object%20Reference) (ButtonPressed :type Key%20Structure :default "AnyKey"))
  ;[1 1 1] Check to see if player has screwdriver equipped. If so delete screw.
  (CallFunction|DestroyScrew (Variables|Default|GetScrew3))
  (CallFunction|CheckAllScrewsDestroyed))

(event OnClicked(Screw2)
  (params (TouchedComponent :type Primitive%20Component%20Object%20Reference) (ButtonPressed :type Key%20Structure :default "AnyKey"))
  ;[1 1 1] Check to see if player has screwdriver equipped. If so delete screw.
  (CallFunction|DestroyScrew (Variables|Default|GetScrew2))
  (CallFunction|CheckAllScrewsDestroyed))

(event OnClicked(Screw4)
  (params (TouchedComponent :type Primitive%20Component%20Object%20Reference) (ButtonPressed :type Key%20Structure :default "AnyKey"))
  ;[1 1 1] Check to see if player has screwdriver equipped. If so delete screw.
  (CallFunction|DestroyScrew (Variables|Default|GetScrew4))
  (CallFunction|CheckAllScrewsDestroyed))

(event OnComponentBeginOverlap(Trigger)
  (params (OverlappedComponent :type Primitive%20Component%20Object%20Reference) (OtherActor :type Actor%20Object%20Reference) (OtherComp :type Primitive%20Component%20Object%20Reference) (OtherBodyIndex :type Integer) (bFromSweep :type Boolean) (SweepResult :type Hit%20Result%20Structure%20%28by%20ref%29))
  (bind _cube (Variables|Default|GetCube))
  ;[1 1 1] Add and Remove UI
  (if (not (or (Variables|Default|GetHaveKey?) (Variables|Default|GetSolved?)))
    (Utilities|IsValid _cube
      (:Is%20Valid
        (Rendering|SetRenderCustomDepth _cube true)
        (bind _returnvalue (UserInterface|CreateWidget "/Game/UI/InteractWidget.InteractWidget_C"))
        (UserInterface|Viewport|AddtoViewport _returnvalue 0)))))

(event OnBeginCursorOver(Screw2)
  (params (TouchedComponent :type Primitive%20Component%20Object%20Reference))
  ;[1 1 1] Highlight Hovered Screws
  (Rendering|SetRenderCustomDepth (Variables|Default|GetScrew2) true))

(event OnComponentEndOverlap(Trigger)
  (params (OverlappedComponent :type Primitive%20Component%20Object%20Reference) (OtherActor :type Actor%20Object%20Reference) (OtherComp :type Primitive%20Component%20Object%20Reference) (OtherBodyIndex :type Integer))
  (bind _cube (Variables|Default|GetCube))
  ;[1 1 1] Add and Remove UI
  (Viewport|RemoveAllWidgets)
  (Utilities|IsValid _cube
    (:Is%20Valid
      (Rendering|SetRenderCustomDepth _cube false))))

(event OnBeginCursorOver(Screw)
  (params (TouchedComponent :type Primitive%20Component%20Object%20Reference))
  ;[1 1 1] Highlight Hovered Screws
  (Rendering|SetRenderCustomDepth (Variables|Default|GetScrew) true))

(event OnEndCursorOver(Screw)
  (params (TouchedComponent :type Primitive%20Component%20Object%20Reference))
  ;[1 1 1] Highlight Hovered Screws
  (Rendering|SetRenderCustomDepth (Variables|Default|GetScrew) false))

(event OnEndCursorOver(Screw2)
  (params (TouchedComponent :type Primitive%20Component%20Object%20Reference))
  ;[1 1 1] Highlight Hovered Screws
  (Rendering|SetRenderCustomDepth (Variables|Default|GetScrew2) false))

(event OnBeginCursorOver(Screw3)
  (params (TouchedComponent :type Primitive%20Component%20Object%20Reference))
  ;[1 1 1] Highlight Hovered Screws
  (Rendering|SetRenderCustomDepth (Variables|Default|GetScrew3) true))

(event OnEndCursorOver(Screw3)
  (params (TouchedComponent :type Primitive%20Component%20Object%20Reference))
  ;[1 1 1] Highlight Hovered Screws
  (Rendering|SetRenderCustomDepth (Variables|Default|GetScrew3) false))

(event OnBeginCursorOver(Screw4)
  (params (TouchedComponent :type Primitive%20Component%20Object%20Reference))
  ;[1 1 1] Highlight Hovered Screws
  (Rendering|SetRenderCustomDepth (Variables|Default|GetScrew4) true))

(event OnEndCursorOver(Screw4)
  (params (TouchedComponent :type Primitive%20Component%20Object%20Reference))
  ;[1 1 1] Highlight Hovered Screws
  (Rendering|SetRenderCustomDepth (Variables|Default|GetScrew4) false))

(event EventBeginPlay
  (CallFunction|CheckifPuzzleWasAlreadySolved))

(event EventOnInteract
  (params (Instigator :type Player%20Character%20Object%20Reference))
  ;[1 1 1] Set camera upon interaction
  (|SetCamera))

(fn ConstructionScript)

(fn CheckAllScrewsDestroyed
  (if (not (Utilities|IsValid (Variables|Default|GetScrew)))
    (if (not (Utilities|IsValid (Variables|Default|GetScrew2)))
      (if (not (Utilities|IsValid (Variables|Default|GetScrew3)))
        (if (not (Utilities|IsValid (Variables|Default|GetScrew4)))
          (Components|DestroyComponent (Variables|Default|GetCube))
          (Variables|Default|SetSolved? true)
          (bind _returnvalue (Game|SpawnActorfromClass "/Game/Blueprints/KeyObject.KeyObject_C" (Math|Transform|MakeTransform "1490.000000,-2550.000000,-290.000000" "0, 0, 0" "0.100000,0.100000,0.100000") "Undefined" 0 0))
          (Variables|/Game/Blueprints/KeyObject.KeyObject_C|SetKeyType _returnvalue "NewEnumerator11"))))))

(fn DestroyScrew
  (params (ScrewComponent :type Static%20Mesh%20Component%20Object%20Reference))
  (LocalVariables|SetLocalMeshComponent ScrewComponent)
  (bind _asmy_game_instance (Utilities|Casting|CastToMyGameInstance (Game|GetGameInstance)))
  (if (Utilities|Enum|Equal(Enum) (Variables|/Game/Blueprints/MyGameInstance.MyGameInstance_C|GetLastClickedItem _asmy_game_instance) (Utilities|Text|MakeLiteralText "Screwdriver"))
    (Components|DestroyComponent (LocalVariables|GetLocalMeshComponent))))

(fn CheckifPuzzleWasAlreadySolved
  (bind _asplayer_character (Utilities|Casting|CastToPlayerCharacter (Game|GetPlayerCharacter 0)))
  (bind _array_element (Utilities|Array|ForEachLoopwithBreak (Variables|/Game/Blueprints/Characters/PlayerCharacter.PlayerCharacter_C|GetOwnedKeys _asplayer_character) :!label _label)
    (:LoopBody
      (if (Utilities|Enum|Equal(Enum) _array_element "NewEnumerator11")
        (Variables|Default|SetHaveKey? true)
        (goto _label Break)))
    (:Completed
      (if (Variables|Default|GetHaveKey?)
        (Components|DestroyComponent (Variables|Default|GetCube))
        (Components|DestroyComponent (Variables|Default|GetScrew))
        (Components|DestroyComponent (Variables|Default|GetScrew2))
        (Components|DestroyComponent (Variables|Default|GetScrew3))
        (Components|DestroyComponent (Variables|Default|GetScrew4))))))