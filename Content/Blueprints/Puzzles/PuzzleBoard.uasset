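; Puzzle board actor with three clickable piece slots, apparently meant to take pieces from the player's inventory.
; Clicking a piece stores its name and mesh, sets its solved flag unconditionally, then checks all three flags, with no action on success.
; Logic for inventory removal, material swaps, restoring slotted pieces on BeginPlay and marking the puzzle solved is present but disconnected, so it never runs.
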(event OnClicked(PuzzlePieceA)
  (params (TouchedComponent :type Primitive%20Component%20Object%20Reference) (ButtonPressed :type Key%20Structure))
  ;[1 1 1] Attempt to Slot Puzzle Piece
  (CallFunction|AddPuzzlePiece (Utilities|Text|MakeLiteralText "Puzzle Piece A") TouchedComponent)
  (Variables|Default|SetASolved? true)
  (CallFunction|CheckPuzzleSolution))

(event OnClicked(PuzzlePieceC)
  (params (TouchedComponent :type Primitive%20Component%20Object%20Reference) (ButtonPressed :type Key%20Structure))
  ;[1 1 1] Attempt to Slot Puzzle Piece
  (CallFunction|AddPuzzlePiece (Utilities|Text|MakeLiteralText "Puzzle Piece C") TouchedComponent)
  (Variables|Default|SetCSolved? true)
  (CallFunction|CheckPuzzleSolution))

(event OnClicked(PuzzlePieceB)
  (params (TouchedComponent :type Primitive%20Component%20Object%20Reference) (ButtonPressed :type Key%20Structure))
  ;[1 1 1] Attempt to Slot Puzzle Piece
  (CallFunction|AddPuzzlePiece (Utilities|Text|MakeLiteralText "Puzzle Piece B") TouchedComponent)
  (Variables|Default|SetBSolved? true)
  (CallFunction|CheckPuzzleSolution))

(event Custom|OnInteract_1)

(event EventBeginPlay
  (CallFunction|SetUpPuzzle))

(fn ConstructionScript)

(fn AddPuzzlePiece
  (params (PuzzleName :type Text) (PuzzleMesh :type Primitive%20Component%20Object%20Reference))
  (LocalVariables|SetClickedPiece PuzzleName)
  (LocalVariables|SetLocalMesh PuzzleMesh))

(fn CheckPuzzleSolution
  (if (Math|Boolean|ANDBoolean (Variables|Default|GetASolved?) (Variables|Default|GetBSolved?) (Variables|Default|GetCSolved?))
    _))

(fn CheckifPuzzleIsSolved
  (Utilities|Casting|CastToPlayerCharacter (Game|GetPlayerCharacter 0)))

(fn SetUpPuzzle)