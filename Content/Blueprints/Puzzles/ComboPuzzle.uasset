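; Interactable combo puzzle actor that grants the player a key.
; Box overlap by the player shows an interact widget and custom-depth highlights the cylinder until they leave.
; OnInteract passes KeyName to CallAppendKeyString if the player is inside the box and HaveKey is false.
; BeginPlay sets HaveKey when the player's OwnedKeys already contain this puzzle's hardcoded key, disabling the prompt and interaction.
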(event OnComponentBeginOverlap(Box)
  (params (OverlappedComponent :type Primitive%20Component%20Object%20Reference) (OtherActor :type Actor%20Object%20Reference) (OtherComp :type Primitive%20Component%20Object%20Reference) (OtherBodyIndex :type Integer) (bFromSweep :type Boolean) (SweepResult :type Hit%20Result%20Structure%20%28by%20ref%29))
  (CallFunction|AddUIandHighlight OtherActor))

(event OnComponentEndOverlap(Box)
  (params (OverlappedComponent :type Primitive%20Component%20Object%20Reference) (OtherActor :type Actor%20Object%20Reference) (OtherComp :type Primitive%20Component%20Object%20Reference) (OtherBodyIndex :type Integer))
  (CallFunction|RemoveUIandHighlight OtherActor))

(event EventOnInteract
  (params (Instigator :type Player%20Character%20Object%20Reference))
  (if (not (Variables|Default|GetHaveKey?))
    (if (Collision|IsOverlappingActor (Variables|Default|GetBox) (Game|GetPlayerCharacter 0) :!class /Script/Engine.PrimitiveComponent)
      (Default|CallAppendKeyString (Variables|Default|GetKeyName)))))

(event EventBeginPlay
  (CallFunction|CheckifPuzzleIsSolved))

(fn ConstructionScript)

(fn DestroyBox
  (Components|DestroyComponent (Variables|Default|GetBox)))

(fn AddUIandHighlight
  (params (Object :type Object%20Object%20Reference))
  (if (== (Utilities|GetClass Object) "/Game/Blueprints/Characters/PlayerCharacter.PlayerCharacter_C")
    (if (not (Variables|Default|GetHaveKey?))
      (bind _returnvalue (UserInterface|CreateWidget "/Game/UI/InteractWidget.InteractWidget_C"))
      (UserInterface|Viewport|AddtoViewport _returnvalue 0)
      (Rendering|SetRenderCustomDepth (Variables|Default|GetCylinder) true))))

(fn RemoveUIandHighlight
  (params (Object :type Object%20Object%20Reference))
  (if (== (Utilities|GetClass Object) "/Game/Blueprints/Characters/PlayerCharacter.PlayerCharacter_C")
    (Viewport|RemoveAllWidgets)
    (Rendering|SetRenderCustomDepth (Variables|Default|GetCylinder) false)))

(fn CheckifPuzzleIsSolved
  (bind _asplayer_character (Utilities|Casting|CastToPlayerCharacter (Game|GetPlayerCharacter 0)))
  (bind _array_element (Utilities|Array|ForEachLoopwithBreak (Variables|/Game/Blueprints/Characters/PlayerCharacter.PlayerCharacter_C|GetOwnedKeys _asplayer_character) :!label _label)
    (:LoopBody
      (if (Utilities|Enum|Equal(Enum) _array_element "NewEnumerator12")
        (Variables|Default|SetHaveKey? true)
        (goto _label Break)))))