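; Three-cube puzzle actor where the player cycles each cube through three heights to earn a key.
; Overlapping a cube's trigger selects it, outlines it via custom depth and shows an interact widget.
; OnInteract raises or wraps the selected cube, then CheckSolution spawns the key and destroys the triggers on the correct combination.
; On BeginPlay, an already owned key places the cubes in solved positions and suppresses trigger prompts.
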(event OnComponentBeginOverlap(LeftTrigger)
  (params (OverlappedComponent :type Primitive%20Component%20Object%20Reference) (OtherActor :type Actor%20Object%20Reference) (OtherComp :type Primitive%20Component%20Object%20Reference) (OtherBodyIndex :type Integer) (bFromSweep :type Boolean) (SweepResult :type Hit%20Result%20Structure%20%28by%20ref%29))
  ;[1 1 1] Toggle UI and Custom Render Depth
  (if (not (Variables|Default|GetHaveKey?))
    (Variables|Default|SetSwitchVariable 0)
    (CallFunction|CreateWidget)
    (Rendering|SetRenderCustomDepth (Variables|Default|GetLeftCube) true)))

(event OnComponentBeginOverlap(MiddleTrigger)
  (params (OverlappedComponent :type Primitive%20Component%20Object%20Reference) (OtherActor :type Actor%20Object%20Reference) (OtherComp :type Primitive%20Component%20Object%20Reference) (OtherBodyIndex :type Integer) (bFromSweep :type Boolean) (SweepResult :type Hit%20Result%20Structure%20%28by%20ref%29))
  ;[1 1 1] Toggle UI and Custom Render Depth
  (if (not (Variables|Default|GetHaveKey?))
    (Variables|Default|SetSwitchVariable 1)
    (CallFunction|CreateWidget)
    (Rendering|SetRenderCustomDepth (Variables|Default|GetMiddleCube) true)))

(event OnComponentBeginOverlap(RightTrigger)
  (params (OverlappedComponent :type Primitive%20Component%20Object%20Reference) (OtherActor :type Actor%20Object%20Reference) (OtherComp :type Primitive%20Component%20Object%20Reference) (OtherBodyIndex :type Integer) (bFromSweep :type Boolean) (SweepResult :type Hit%20Result%20Structure%20%28by%20ref%29))
  ;[1 1 1] Toggle UI and Custom Render Depth
  (if (not (Variables|Default|GetHaveKey?))
    (Variables|Default|SetSwitchVariable 2)
    (CallFunction|CreateWidget)
    (Rendering|SetRenderCustomDepth (Variables|Default|GetRightCube) true)))

(event OnComponentEndOverlap(LeftTrigger)
  (params (OverlappedComponent :type Primitive%20Component%20Object%20Reference) (OtherActor :type Actor%20Object%20Reference) (OtherComp :type Primitive%20Component%20Object%20Reference) (OtherBodyIndex :type Integer))
  ;[1 1 1] Toggle UI and Custom Render Depth
  (Rendering|SetRenderCustomDepth (Variables|Default|GetLeftCube) false)
  (bind _boolean (CallFunction|RemoveWidget))
  (if _boolean
    (Variables|Default|SetSwitchVariable -1)))

(event OnComponentEndOverlap(MiddleTrigger)
  (params (OverlappedComponent :type Primitive%20Component%20Object%20Reference) (OtherActor :type Actor%20Object%20Reference) (OtherComp :type Primitive%20Component%20Object%20Reference) (OtherBodyIndex :type Integer))
  ;[1 1 1] Toggle UI and Custom Render Depth
  (Rendering|SetRenderCustomDepth (Variables|Default|GetMiddleCube) false)
  (bind _boolean (CallFunction|RemoveWidget))
  (if _boolean
    (Variables|Default|SetSwitchVariable -1)))

(event OnComponentEndOverlap(RightTrigger)
  (params (OverlappedComponent :type Primitive%20Component%20Object%20Reference) (OtherActor :type Actor%20Object%20Reference) (OtherComp :type Primitive%20Component%20Object%20Reference) (OtherBodyIndex :type Integer))
  ;[1 1 1] Toggle UI and Custom Render Depth
  (Rendering|SetRenderCustomDepth (Variables|Default|GetRightCube) false)
  (bind _boolean (CallFunction|RemoveWidget))
  (if _boolean
    (Variables|Default|SetSwitchVariable -1)))

(event EventOnInteract
  (params (Instigator :type Player%20Character%20Object%20Reference))
  ;[1 1 1] Set orientation of Cubes
  (switch int (Variables|Default|GetSwitchVariable)
    (:0
      (bind _output_integar (CallFunction|SetOrientation (Variables|Default|GetLeftCube) (Variables|Default|GetLeftCubePosition)))
      (bind _output_get (Variables|Default|SetLeftCubePosition _output_integar)))
    (:1
      (bind _output_integar_2 (CallFunction|SetOrientation (Variables|Default|GetMiddleCube) (Variables|Default|GetMiddleCubePosition)))
      (bind _output_get_2 (Variables|Default|SetMiddleCubePosition _output_integar_2)))
    (:2
      (bind _output_integar_3 (CallFunction|SetOrientation (Variables|Default|GetRightCube) (Variables|Default|GetRightCubePosition)))
      (bind _output_get_3 (Variables|Default|SetRightCubePosition _output_integar_3))))
  (CallFunction|CheckSolution _output_get _output_get_2 _output_get_3))

(event EventBeginPlay
  (CallFunction|CheckforKey))

(fn ConstructionScript)

(fn SetOrientation
  (params (StaticMeshComponent :type Static%20Mesh%20Component%20Object%20Reference) (LocalIntegar :type Integer))
  (LocalVariables|SetLocal_StaticMeshComponent StaticMeshComponent)
  (LocalVariables|SetLocal_Int LocalIntegar)
  (if (== (LocalVariables|GetLocal_Int) 2)
    (Class|SceneComponent|AddWorldTransform (LocalVariables|GetLocal_StaticMeshComponent) (Math|Transform|MakeTransform "0, 0,-100.000000" "0.000000, 0, 0" "1,1.000000,1") false false)
    (LocalVariables|SetLocal_Int 0)
    (else
      (Class|SceneComponent|AddWorldTransform (LocalVariables|GetLocal_StaticMeshComponent) (Math|Transform|MakeTransform "0, 0,50.000000" "0.000000, 0, 0" "1,1.000000,1") false false)
      (Math|Integer|IncrementInt (LocalVariables|GetLocal_Int)
        (:%20%20
          _))))
  (return (LocalVariables|GetLocal_Int)))

(fn CheckSolution
  (params (LeftCubePosition :type Integer) (MiddleCubePosition :type Integer) (RightCubePosition :type Integer))
  (Utilities|FlowControl|Sequence
    (:then_0
      (LocalVariables|SetLocal_LeftInt LeftCubePosition)
      (LocalVariables|SetLocal_MiddleInt MiddleCubePosition)
      (LocalVariables|SetLocal_RightInt RightCubePosition))
    (:then_1
      (if (Math|Boolean|ANDBoolean (== (LocalVariables|GetLocal_LeftInt) 1) (== (LocalVariables|GetLocal_MiddleInt) 2) (== (LocalVariables|GetLocal_RightInt) 0))
        (bind _returnvalue (Game|SpawnActorfromClass "/Game/Blueprints/KeyObject.KeyObject_C" (Math|Transform|MakeTransform "1795.000000,-1480.000000,-285.000000" "0, 0, 0" "0.300000,0.300000,0.300000") "Undefined" 0 0))
        (Variables|/Game/Blueprints/KeyObject.KeyObject_C|SetKeyType _returnvalue "NewEnumerator10")
        (Components|DestroyComponent (Variables|Default|GetLeftTrigger))
        (Components|DestroyComponent (Variables|Default|GetMiddleTrigger))
        (Components|DestroyComponent (Variables|Default|GetRightTrigger))))))

(fn RemoveWidget
  (bind _returnvalue (Game|GetPlayerCharacter 0))
  (bind _lefttrigger (Variables|Default|GetLeftTrigger))
  (bind _righttrigger (Variables|Default|GetRightTrigger))
  (bind _middletrigger (Variables|Default|GetMiddleTrigger))
  (bind _capsulecomponent (Variables|/Script/Engine.Character|GetCapsuleComponent _returnvalue))
  (bind _returnvalue_2 (Class|PrimitiveComponent|IsOverlappingComponent _capsulecomponent _middletrigger))
  (bind _returnvalue_3 (Class|PrimitiveComponent|IsOverlappingComponent _capsulecomponent _lefttrigger))
  (bind _returnvalue_4 (Class|PrimitiveComponent|IsOverlappingComponent _capsulecomponent _righttrigger))
  (bind _returnvalue_5 (Math|Boolean|ORBoolean _returnvalue_3 _returnvalue_4 _returnvalue_2))
  (Utilities|IsValid _returnvalue
    (:Is%20Valid
      (if (not _returnvalue_5)
        (Viewport|RemoveAllWidgets)
        (return _returnvalue_5)))))

(fn CreateWidget
  (bind _returnvalue (UserInterface|CreateWidget "/Game/UI/InteractWidget.InteractWidget_C"))
  (UserInterface|Viewport|AddtoViewport _returnvalue 0))

(fn CheckforKey
  (bind _asplayer_character (Utilities|Casting|CastToPlayerCharacter (Game|GetPlayerCharacter 0)))
  (bind _array_element (Utilities|Array|ForEachLoopwithBreak (Variables|/Game/Blueprints/Characters/PlayerCharacter.PlayerCharacter_C|GetOwnedKeys _asplayer_character) :!label _label)
    (:LoopBody
      (if (Utilities|Enum|Equal(Enum) _array_element "NewEnumerator10")
        (Variables|Default|SetHaveKey? true)
        (Class|SceneComponent|AddWorldTransform (Variables|Default|GetLeftCube) (Math|Transform|MakeTransform "0, 0,50.000000" "0, 0, 0" "1,1,1") false false)
        (Class|SceneComponent|AddWorldTransform (Variables|Default|GetMiddleCube) (Math|Transform|MakeTransform "0, 0,100.000000" "0, 0, 0" "1,1,1") false false)
        (goto _label Break)))))